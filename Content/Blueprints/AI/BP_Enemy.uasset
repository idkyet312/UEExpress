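; BP_Enemy is a hostile actor that faces the player's train engine and fires rockets at it.
; On BeginPlay it casts the player pawn to BP_TrainEnginePawn, caches it and starts a looping timer that calls Shoot.
; Tick rotates StaticMesh toward the TrainEngine component every frame, without checking that the cached pawn is valid.
; Shoot spawns a BP_Rocket at the Aimwith component, oriented along its forward vector.
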(event `ShootAtTrain`
  (`self.Shoot`))

(event `self.ReceiveBeginPlay`
  (bind _asbp_train_engine_pawn (cast `/Game/LevelPrototyping/Blueprints/BP_TrainEnginePawn` (`GameplayStatics.GetPlayerPawn` 0))
    (:`then`
      (set `self.As BP Train Engine Pawn` _asbp_train_engine_pawn)
      (`KismetSystemLibrary.K2_SetTimerDelegate` (delegate `ShootAtTrain`) 3.0 true)
      (`KismetSystemLibrary.PrintString` "Enemy ready"))
    (:`CastFailed`
      (`KismetSystemLibrary.PrintString` "Hello"))))

(event `self.ReceiveTick`
  (params (DeltaSeconds :type "Float (single-precision)"))
  (`SceneComponent.K2_SetWorldRotation` (`self.StaticMesh`) (`KismetMathLibrary.FindLookAtRotation` (`SceneComponent.K2_GetComponentLocation` (`self.StaticMesh`)) (`SceneComponent.K2_GetComponentLocation` (`/Game/LevelPrototyping/Blueprints/BP_TrainEnginePawn.TrainEngine` (`self.As BP Train Engine Pawn`)))) false false))

(fn `Shoot`
  (bind _aimwith (`self.aimwith`))
  (`|SpawnActorFromClass` "/Game/Blueprints/AI/weapons/BP_Rocket.BP_Rocket_C" (`KismetMathLibrary.MakeTransform` (`SceneComponent.K2_GetComponentLocation` _aimwith) (`KismetMathLibrary.Conv_VectorToRotator` (`SceneComponent.GetForwardVector` _aimwith))) "AlwaysSpawn" "MultiplyWithRoot" null null))

(fn `UserConstructionScript`)